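; Player controller that sets up input and the on-screen HUD and tracks a score.
; On BeginPlay it adds an Enhanced Input mapping context, then creates the main widget and adds it to the viewport.
; UpdateScore increments the score by one and writes it directly to the widget's score text.
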(event `self.ReceiveBeginPlay`
  ; Forma de inicializar los inputs
  (`EnhancedInputSubsystemInterface.AddMappingContext` (subsystem `EnhancedInputLocalPlayerSubsystem`) "/Game/MyContent/BPs/Inputs/MappingContext.MappingContext" 0 (struct))
  ; INTERFACE
  (bind _returnvalue (`|CreateWidget` "/Game/MyContent/BPs/UI/WBP_MainWidget.WBP_MainWidget_C" self))
  (bind _output_get (set `self.MyWidget` _returnvalue))
  (`UserWidget.AddToViewport` _output_get 0))

(fn `UpdateScore`
  (bind _output_get (set `self.Score` (+ (`self.Score`) 1)))
  (`TextBlock.SetText` (`/Game/MyContent/BPs/UI/WBP_MainWidget.ScoreText_1` (`self.MyWidget`)) (`KismetTextLibrary.Conv_StringToText` (`KismetStringLibrary.Concat_StrStr` "" (`KismetStringLibrary.Conv_IntToString` _output_get)))))

(fn `UserConstructionScript`)