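; BP_PlayerPawn is the player pawn of a coin-collecting level game, moved by Enhanced Input through swept, normalized local offsets scaled by speed and delta time.
; Tag-checked overlaps destroy coins and update the controller's score, which gates Exit to MyLevel2 and GameExit to FinalMenus.
; Any other overlap calls Death, which reloads the current level and creates a death widget.
; Position-reset nodes are left unconnected.
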(event `self.ReceiveBeginPlay`
  ; TE BUSCA EN LA ESCENA
  (bind _returnvalue (`GameplayStatics.GetActorOfClass` "/Script/Engine.PlayerStart"))
  (set `self.InitLocation` (`self.K2_GetActorLocation` _returnvalue)))

(event `self.ReceiveActorBeginOverlap`
  (params (OtherActor :type "Actor Object Reference"))
  (bind _returnvalue (`self.ActorHasTag` OtherActor "Coin"))
  ; OnTriggerEnd
  (if _returnvalue
    (if _returnvalue
      (`self.K2_DestroyActor` OtherActor)
      (bind _asbp_my_player_controllerr (cast `/Game/MyContent/BPs/Frameworks/BP_MyPlayerControllerr` (`self.GetController`)))
      (`/Game/MyContent/BPs/Frameworks/BP_MyPlayerControllerr.UpdateScore` _asbp_my_player_controllerr)
      (else
        (`self.Death` :!label _label)))
    (else
      ; PARA QUE ABRA EL SEGUNDO NIVEL
      (if (`self.ActorHasTag` OtherActor "Exit")
        (bind _asbp_player_pawn (cast `/Game/MyContent/BPs/Objects/BP_PlayerPawn` self))
        (bind _asbp_my_player_controllerr_2 (cast `/Game/MyContent/BPs/Frameworks/BP_MyPlayerControllerr` (`self.GetController` _asbp_player_pawn)))
        (if (>= (`/Game/MyContent/BPs/Frameworks/BP_MyPlayerControllerr.Score` _asbp_my_player_controllerr_2) (`/Game/MyContent/BPs/Frameworks/BP_MyPlayerControllerr.TotalCoins` _asbp_my_player_controllerr_2))
          (`GameplayStatics.OpenLevelBySoftObjectPtr` "/Game/MyContent/Levels/MyLevel2.MyLevel2")
          (else
            (`KismetSystemLibrary.PrintString` "TODAVIA TE QUEDAN MONEDAS!!!" true true (struct :`R` 1.0 :`G` 0.034048 :`A` 1.0))))
        (elif (`self.ActorHasTag` OtherActor "GameExit")
          (bind _asbp_player_pawn_2 (cast `/Game/MyContent/BPs/Objects/BP_PlayerPawn` self))
          (bind _asbp_my_player_controllerr_3 (cast `/Game/MyContent/BPs/Frameworks/BP_MyPlayerControllerr` (`self.GetController` _asbp_player_pawn_2)))
          (if (>= (`/Game/MyContent/BPs/Frameworks/BP_MyPlayerControllerr.Score` _asbp_my_player_controllerr_3) (`/Game/MyContent/BPs/Frameworks/BP_MyPlayerControllerr.TotalCoins` _asbp_my_player_controllerr_3))
            (`GameplayStatics.OpenLevelBySoftObjectPtr` "/Game/MyContent/Levels/FinalMenus.FinalMenus")
            (else
              (`KismetSystemLibrary.PrintString` "TODAVIA TE QUEDAN MONEDAS!!!" true true (struct :`R` 1.0 :`G` 0.034048 :`A` 1.0))))
          (else
            (goto _label)))))))

(event `EnhancedInput|/Game/MyContent/BPs/Inputs/MoveAction`
  (params (ActionValue :type "Vector2D Structure") (ElapsedSeconds :type "Float (double-precision)") (TriggeredSeconds :type "Float (double-precision)") (InputAction :type "InputAction Object Reference" :default "/Game/MyContent/BPs/Inputs/MoveAction.MoveAction"))
  ; Este evento se ejecuta cuando se realiza una acción
  (:`Triggered`
    (`self.K2_AddActorLocalOffset` (* (`KismetMathLibrary.Normal2D` ActionValue) (`self.velocidad`) (`GameplayStatics.GetWorldDeltaSeconds`)) true)))

(event `self.ReceiveTick`
  (params (DeltaSeconds :type "Float (single-precision)")))

(fn `Death`
  (bind _returnvalue (`GameplayStatics.GetCurrentLevelName` true))
  (`GameplayStatics.OpenLevel` (`KismetStringLibrary.Conv_StringToName` _returnvalue))
  (bind _returnvalue_2 (`|CreateWidget` "/Game/MyContent/BPs/UI/WBP_DeathImage.WBP_DeathImage_C"))
  (`UserWidget.AddToViewport` _returnvalue_2 1))

(fn `UserConstructionScript`)

(fn `x3`
  (params (A :type "Float (double-precision)"))
  ;[0 0.02073 0.15 0.5 16] Comentario
  (bind _output_get (set `self.MyPoints` (+ (`self.MyPoints`) (* A 3.0))))
  (`KismetSystemLibrary.PrintString` (`KismetStringLibrary.Conv_DoubleToString` _output_get)))