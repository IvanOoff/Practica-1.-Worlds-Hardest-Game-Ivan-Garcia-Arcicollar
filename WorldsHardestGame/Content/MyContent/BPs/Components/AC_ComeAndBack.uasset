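; AC_ComeAndBack is an actor component that moves its owner back and forth in a straight line.
; Tick offsets the owner in local space by the Vel and Dir variables scaled by delta time, without sweeping for collisions.
; A looping timer started on BeginPlay negates Vel every two seconds to reverse the motion.
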(event `self.ReceiveBeginPlay`
  (`KismetSystemLibrary.K2_SetTimerDelegate` (delegate `OnTimerEnd`) 2.0 true))

(event `OnTimerEnd`
  (set `self.vel` (* -1.0 (`self.vel`))))

(event `self.ReceiveTick`
  (params (DeltaSeconds :type "Float (single-precision)"))
  (`Actor.K2_AddActorLocalOffset` (`self.GetOwner`) (* DeltaSeconds (`self.vel`) (`self.dir`)) false false))